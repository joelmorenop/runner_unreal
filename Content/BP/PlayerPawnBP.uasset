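; Player pawn that moves on the X/Y plane from Forward, Backward, Left and Right input actions.
; Input events set held-direction flags, which Tick reads to set the Mesh's physics linear velocity through MoveActor.
; Each call replaces the velocity, so directions do not combine and the last one checked wins.
; BeginPlay holds Speed at zero for Duration seconds, then restores and prints it.
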(event EventBeginPlay
  (Variables|Default|SetinitialSpeed (Variables|Default|Getspeed))
  (Variables|Default|Setspeed 0)
  (Utilities|FlowControl|Delay (Math|Conversions|ToFloat(Integer) (Variables|Default|GetDuration)))
  (bind _output_get (Variables|Default|Setspeed (Variables|Default|GetinitialSpeed)))
  (Development|PrintString (Utilities|String|ToString(Float) (Math|Conversions|ToFloat(Integer) _output_get))))

(event Collision|EventActorBeginOverlap
  (params (OtherActor :type Actor%20Object%20Reference)))

(event EventTick
  (params (DeltaSeconds :type Float%20%28single-precision%29))
  (bind _speed (Variables|Default|Getspeed))
  (bind _returnvalue (* _speed -1))
  (Utilities|FlowControl|Sequence
    (:then_0
      (if (Variables|Default|GetRightPressed)
        (CallFunction|MoveActor _speed)))
    (:then_1
      (if (Variables|Default|GetLeftPressed)
        (CallFunction|MoveActor _returnvalue)))
    (:then_2
      (if (Variables|Default|GetForwardPressed)
        (CallFunction|MoveActor 0 _speed)))
    (:then_3
      (if (Variables|Default|GetBackwardPressed)
        (CallFunction|MoveActor 0 _returnvalue)))))

(event Input|ActionEvents|InputActionForward
  (params (Key :type Key%20Structure :default "None"))
  ;[1 1 1] Controls
  (:Pressed
    (Variables|Default|SetForwardPressed true))
  (:Released
    (Variables|Default|SetForwardPressed false)))

(event Input|ActionEvents|InputActionLeft
  (params (Key :type Key%20Structure :default "None"))
  ;[1 1 1] Controls
  (:Pressed
    (Variables|Default|SetLeftPressed true))
  (:Released
    (Variables|Default|SetLeftPressed false)))

(event Input|ActionEvents|InputActionRight
  (params (Key :type Key%20Structure :default "None"))
  ;[1 1 1] Controls
  (:Pressed
    (Variables|Default|SetRightPressed true))
  (:Released
    (Variables|Default|SetRightPressed false)))

(event Input|ActionEvents|InputActionBackward
  (params (Key :type Key%20Structure :default "None"))
  ;[1 1 1] Controls
  (:Pressed
    (Variables|Default|SetBackwardPressed true))
  (:Released
    (Variables|Default|SetBackwardPressed false)))

(fn ConstructionScript)

(fn MoveActor
  (params (X :type Integer) (Y :type Integer))
  (Physics|SetPhysicsLinearVelocity (Variables|Default|GetMesh) (Math|Vector|MakeVector (Math|Conversions|ToFloat(Integer) X) (Math|Conversions|ToFloat(Integer) Y) 0.0) false "None"))