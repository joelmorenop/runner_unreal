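; Input-driven actor Blueprint that tracks four directional controls and holds its speed at zero for a startup delay.
; BeginPlay zeroes Speed, waits for Duration, then restores it to InitialSpeed.
; Forward, Backward, Left and Right input actions set and clear matching pressed flags.
; Nothing here reads those flags or Speed: Tick is disabled and MoveActor is an empty stub, so no movement is applied.
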(event EventBeginPlay
  (Variables|Default|SetinitialSpeed (Variables|Default|GetinitialSpeed))
  (Variables|Default|Setspeed 0.0)
  (Utilities|FlowControl|Delay (Variables|Default|GetDuration))
  (Variables|Default|Setspeed (Variables|Default|GetinitialSpeed)))

(event Collision|EventActorBeginOverlap
  (params (OtherActor :type Actor%20Object%20Reference)))

(event EventTick
  (params (DeltaSeconds :type Float%20%28single-precision%29)))

(event Input|ActionEvents|InputActionForward
  (params (Key :type Key%20Structure :default "None"))
  (:Pressed
    (Variables|Default|SetForwardPressed true))
  (:Released
    (Variables|Default|SetForwardPressed false)))

(event Input|ActionEvents|InputActionLeft
  (params (Key :type Key%20Structure :default "None"))
  (:Pressed
    (Variables|Default|SetLeftPressed true))
  (:Released
    (Variables|Default|SetLeftPressed false)))

(event Input|ActionEvents|InputActionRight
  (params (Key :type Key%20Structure :default "None"))
  (:Pressed
    (Variables|Default|SetRightPressed true))
  (:Released
    (Variables|Default|SetRightPressed false)))

(event Input|ActionEvents|InputActionBackward
  (params (Key :type Key%20Structure :default "None"))
  (:Pressed
    (Variables|Default|SetBackwardPressed true))
  (:Released
    (Variables|Default|SetBackwardPressed false)))

(fn ConstructionScript)

(fn MoveActor
  (params (X :type Integer) (Y :type Integer)))