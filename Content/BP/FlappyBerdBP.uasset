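; FlappyBerdBP is the player bird for a Flappy Bird-style game, handling jumping, death and scoring.
; While the bird is alive, Jump calls MoveFlappy, which zeroes the capsule's physics velocity before adding an upward force for consistent flaps.
; Capsule overlaps check component tags: "pipe" kills the bird and destroys its capsule and sprite.
; A "point" tag increments Score and updates the HUD through the cached GMBBP game mode.
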(event OnComponentBeginOverlap(Capsule)
  (params (OverlappedComponent :type Primitive%20Component%20Object%20Reference) (OtherActor :type Actor%20Object%20Reference) (OtherComp :type Primitive%20Component%20Object%20Reference) (OtherBodyIndex :type Integer) (bFromSweep :type Boolean) (SweepResult :type Hit%20Result%20Structure%20%28by%20ref%29))
  (bind _gmbbp (Variables|Default|GetGMBBP))
  (bind _hud (Variables|/Game/BP/GMBBP.GMBBP_C|GetHUD _gmbbp))
  ;[1 1 1] If flappy gets hit he dies
  (if (Components|ComponentHasTag OtherComp "pipe")
    (bind _output_get (Variables|Default|SetAlive false))
    (Development|PrintString (Utilities|String|ToString(Boolean) _output_get))
    (Components|DestroyComponent (Variables|Default|GetCapsule))
    (Components|DestroyComponent (Variables|Default|GetPaperSprite))
    (else
      ;[1 0.4849 0.3748] If flappy does not get hit + pass the pipe, flappy gets a point :D
      (if (Components|ComponentHasTag OtherComp "point")
        (bind _output_get_2 (Variables|Default|SetScore (+ (stale _output_get_2) 1)))
        (Utilities|IsValid _hud
          (:Is%20Valid
            (Default|SetPoints _hud _output_get_2)))))))

(event EventBeginPlay
  ;[1 1 1] Get a game mode reference
  (bind _asgmbbp (Utilities|Casting|CastToGMBBP (Game|GetGameMode)))
  (Variables|Default|SetGMBBP _asgmbbp))

(event Collision|EventActorBeginOverlap
  (params (OtherActor :type Actor%20Object%20Reference)))

(event EventTick
  (params (DeltaSeconds :type Float%20%28single-precision%29)))

(event Input|ActionEvents|InputActionJump
  (params (Key :type Key%20Structure))
  ;[1 1 1] Flappy jump, if flappy is alive then jump
  (:Pressed
    (if (Variables|Default|GetAlive)
      (CallFunction|MoveFlappy))))

(fn ConstructionScript)

(fn MoveFlappy
  (bind _capsule (Variables|Default|GetCapsule))
  ;[1 1 1] Add jump force to flappy capsule
  (Physics|SetPhysicsLinearVelocity _capsule "0, 0, 0" false "None")
  (Physics|AddForce _capsule (Math|Vector|MakeVector 0.0 0.0 (Variables|Default|GetJumpForce)) "None" false))